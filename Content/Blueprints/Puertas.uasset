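; Sliding door Blueprint that rises when an actor overlaps it and lowers again after a pause.
; MoverPuerta and CerrarPuerta move the Cube in fixed local Z steps through delayed self-calls, stopping at hard-coded world heights.
; The Mover flag halts closing when a new overlap reopens the door.
; Metal open and close sounds spawn at the world origin rather than at the door.
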(event `self.ReceiveActorBeginOverlap`
  (params (OtherActor :type "Actor Object Reference"))
  (set `self.mover` true)
  (`self.Mover Puerta`)
  (`GameplayStatics.SpawnSoundAtLocation` "/Game/Sonidos/SFX/Puertas/puerta_metal_abrir_arriba.puerta_metal_abrir_arriba" (0.0 0.0 0.0) (struct) 1.0 1.0 0.0 null null))

(event `Mover Puerta`
  (bind (_returnvalue_x _returnvalue_y _returnvalue_z) (`KismetMathLibrary.BreakVector` (`SceneComponent.K2_GetComponentLocation` (`self.Cube`))))
  (if (< _returnvalue_z 850.0)
    (`SceneComponent.K2_AddLocalOffset` (`self.Cube`) (0.0 0.0 20.0) false false)
    (`KismetSystemLibrary.Delay` 0.1)
    (`self.Mover Puerta`)
    (else
      (set `self.mover` false)
      (`KismetSystemLibrary.Delay` 5.0)
      (`self.Cerrar Puerta`)
      (`GameplayStatics.SpawnSoundAtLocation` "/Game/Sonidos/SFX/Puertas/puerta_metal_cerrar_arriba.puerta_metal_cerrar_arriba" (0.0 0.0 0.0) (struct) 1.0 1.0 0.0 null null))))

(event `Cerrar Puerta`
  (bind (_returnvalue_x _returnvalue_y _returnvalue_z) (`KismetMathLibrary.BreakVector` (`SceneComponent.K2_GetComponentLocation` (`self.Cube`))))
  (if (`self.mover`)
    _
    (elif (> _returnvalue_z 400.0)
      (`SceneComponent.K2_AddLocalOffset` (`self.Cube`) (0.0 0.0 -20.0) false false)
      (`KismetSystemLibrary.Delay` 0.1)
      (`self.Cerrar Puerta`))))

(fn `UserConstructionScript`)